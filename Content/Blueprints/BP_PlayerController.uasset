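; Player controller for a voxel block game that creates the HUD and handles breaking, placing and picking blocks.
; A debug-drawn camera line trace finds the ChunkBase under view, offsetting the hit by its normal to resolve the local block position.
; Left click sets the block to Air, right click places CurrentBlockType on the adjacent face, and middle click copies the block type.
; Bedrock cannot be broken or picked.
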(event EventBeginPlay
  (bind _returnvalue (UserInterface|CreateWidget "/Game/Blueprints/WBP_HUD.WBP_HUD_C"))
  (UserInterface|Viewport|AddtoViewport _returnvalue 0))

(event Input|MouseEvents|RightMouseButton
  (params (Key :type Key%20Structure :default "None"))
  (:Pressed
    (bind (_returnvalue _outhit) (CallFunction|Raycast))
    (if _returnvalue
      (bind _aschunk_base (Utilities|Casting|CastToChunkBase (.HitActor (Collision|BreakHitResult _outhit))))
      (Class|ChunkBase|ModifyVoxel _aschunk_base (Class|KismetMathLibrary|FTruncVector (+ (Class|VoxelFunctionLibrary|WorldtoLocalBlockPosition (- (.Location (Collision|BreakHitResult _outhit)) (.Normal (Collision|BreakHitResult _outhit))) (Variables|Default|GetChunkSize)) (.Normal (Collision|BreakHitResult _outhit)))) (Variables|Default|GetCurrentBlockType)))))

(event Input|MouseEvents|LeftMouseButton
  (params (Key :type Key%20Structure :default "None"))
  (:Pressed
    (bind (_returnvalue _outhit) (CallFunction|Raycast))
    (if _returnvalue
      (bind _aschunk_base (Utilities|Casting|CastToChunkBase (.HitActor (Collision|BreakHitResult _outhit))))
      (if (Utilities|Enum|NotEqual(Enum) (Class|ChunkBase|GetBlock _aschunk_base (Class|VoxelFunctionLibrary|WorldtoLocalBlockPosition (- (.Location (Collision|BreakHitResult _outhit)) (.Normal (Collision|BreakHitResult _outhit))) (Variables|Default|GetChunkSize))) "Bedrock")
        (Class|ChunkBase|ModifyVoxel _aschunk_base (Class|VoxelFunctionLibrary|WorldtoLocalBlockPosition (- (.Location (Collision|BreakHitResult _outhit)) (.Normal (Collision|BreakHitResult _outhit))) (Variables|Default|GetChunkSize)) "Air")))))

(event Input|MouseEvents|MiddleMouseButton
  (params (Key :type Key%20Structure :default "None"))
  (:Pressed
    (bind (_returnvalue _outhit) (CallFunction|Raycast))
    (if _returnvalue
      (bind _aschunk_base (Utilities|Casting|CastToChunkBase (.HitActor (Collision|BreakHitResult _outhit))))
      (if (Utilities|Enum|NotEqual(Enum) (Class|ChunkBase|GetBlock _aschunk_base (Class|VoxelFunctionLibrary|WorldtoLocalBlockPosition (- (.Location (Collision|BreakHitResult _outhit)) (.Normal (Collision|BreakHitResult _outhit))) (Variables|Default|GetChunkSize))) "Bedrock")
        (bind _output_get (Variables|Default|SetCurrentBlockType (Class|ChunkBase|GetBlock _aschunk_base (Class|VoxelFunctionLibrary|WorldtoLocalBlockPosition (- (.Location (Collision|BreakHitResult _outhit)) (.Normal (Collision|BreakHitResult _outhit))) (Variables|Default|GetChunkSize)))))
        (Development|PrintString (Utilities|String|EnumtoString _output_get) true true "(R=0.107346,G=0.692708,B=0.110839,A=1.000000)")))))

(fn ConstructionScript)

(fn Raycast
  (bind _playercameramanager (Variables|Default|GetPlayerCameraManager))
  (bind _returnvalue (Camera|GetCameraLocation _playercameramanager))
  (bind (_outhit _returnvalue_2) (Collision|LineTraceByChannel _returnvalue (+ _returnvalue (* (Math|Vector|GetForwardVector (Camera|GetCameraRotation _playercameramanager)) (Variables|Default|GetBlockDistance))) "TraceTypeQuery1" false 0 "ForDuration" true "(R=1.000000,G=0.000000,B=0.000000,A=1.000000)" "(R=0.000000,G=1.000000,B=0.000000,A=1.000000)" 1e+01))
  (return _returnvalue_2 _outhit))