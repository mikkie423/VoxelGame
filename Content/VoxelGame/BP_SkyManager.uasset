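; Sky manager for the voxel game, handling day/night, sun and moon motion, calendar, seasons and weather.
; Tick advances the clocks, rotates sun and moon with eased interpolation, and shows stars at evening and night.
; The month sets season and sunrise/sunset times; season weights build randomized hourly rain and snow schedules that toggle effects.
; Stars, rain and snow attach to the player pawn, with stars keeping absolute rotation.
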(event Custom|ToggleStardome
  (bind _partofday (CallFunction|GetPartOfDay))
  (bind _partofday_2 (CallFunction|GetPartOfDay))
  (if (!= (Variables|Default|GetbShowStardome) (or (Utilities|Enum|Equal(Enum) _partofday_2 "NewEnumerator2") (Utilities|Enum|Equal(Enum) _partofday_2 "NewEnumerator3")))
    (bind _output_get (Variables|Default|SetbShowStardome (or (Utilities|Enum|Equal(Enum) _partofday "NewEnumerator2") (Utilities|Enum|Equal(Enum) _partofday "NewEnumerator3"))))
    (if _output_get
      (Components|Activation|Activate (Variables|Default|GetStars) false)
      (else
        (Components|Activation|Deactivate (Variables|Default|GetStars))))))

(event Custom|CheckPlayerReady
  (Utilities|IsValid (Game|Player|GetPlayerPawn 0)
    (:Is%20Valid
      (Utilities|Time|ClearandInvalidateTimerbyHandle (Variables|Default|GetCheckPlayerReadyTimer))
      (Transformation|AttachComponentToComponent (Variables|Default|GetStars) (Variables|/Script/Engine.Actor|GetRootComponent (Game|Player|GetPlayerPawn 0)) "None" "SnapToTarget" "KeepRelative" "KeepRelative" true)
      (Transformation|SetAbsolute (Variables|Default|GetStars) false true false)
      (CallFunction|InitStardome))))

(event Custom|AttachWeather
  (Transformation|AttachComponentToComponent (Variables|Default|GetRainComponent) (Variables|/Script/Engine.Actor|GetRootComponent (Game|Player|GetPlayerPawn 0)) "None" "SnapToTarget" "KeepRelative" "KeepRelative" true)
  (Development|PrintString "Rain Attached")
  (Transformation|AttachComponentToComponent (Variables|Default|GetSnowComponent) (Variables|/Script/Engine.Actor|GetRootComponent (Game|Player|GetPlayerPawn 0)) "None" "SnapToTarget" "KeepRelative" "KeepRelative" true)
  (Development|PrintString "Snow Attached"))

(event EventBeginPlay
  (bind _returnvalue (Utilities|Time|SetTimerbyEvent (EventDispatchers|CreateEvent :!event Custom|CheckPlayerReady) 0.2 true))
  (Variables|Default|SetCheckPlayerReadyTimer _returnvalue)
  (if (Variables|Default|GetbHasTime)
    (Utilities|Time|SetTimerbyEvent (EventDispatchers|CreateEvent :!event UpdateDate) (* (Variables|TimeSetup|GetDayLength) 6e+01) true)
    (else
      (Development|PrintString "Has No Time")))
  (if (Variables|Default|GetbHasWeather)
    (Utilities|FlowControl|Sequence
      (:then_0
        (CallFunction|AttachWeather)
        (Development|PrintString "Attaching Weather"))
      (:then_1
        (bind _returnvalue_2 (Utilities|Time|SetTimerbyEvent (EventDispatchers|CreateEvent :!event UpdateWeather) (Variables|TimeSetup|GetUpdateFrequency) true))
        (Variables|Precipitation|SetUpdateWeatherTimer _returnvalue_2)
        (Class|BPIWeatherSystem|CreateTimeWidget(Message) (Game|GetPlayerController 0) self :!label _label)))
    (else
      (Development|PrintString "Has No Weather")
      (goto _label))))

(event EventTick
  (params (DeltaSeconds :type Float%20%28single-precision%29))
  (if (Variables|Default|GetbHasTime)
    (CallFunction|ComputeCurrentTime)
    (CallFunction|UpdateSunMoonPosition (Utilities|Select :Index (Variables|Season|GetSeason) :NewEnumerator0 2.1e+02 :NewEnumerator1 225.0 :NewEnumerator2 2.1e+02 :NewEnumerator3 195.0))
    (CallFunction|ToggleStardome)))

(fn ConstructionScript
  (if (Variables|Default|GetbEditorLaunchRefresh)
    (Variables|Default|SetbEditorLaunchRefresh false))
  (if (Variables|Default|GetbHasTime)
    (CallFunction|UpdateSunMoonPosition (Utilities|Select :Index (Variables|Season|GetSeason) :NewEnumerator0 2.1e+02 :NewEnumerator1 225.0 :NewEnumerator2 2.1e+02 :NewEnumerator3 195.0)))
  (CallFunction|InitStardome)
  (Components|Activation|SetAutoActivate (Variables|Default|GetStars) false)
  (CallFunction|UpdateDate)
  (CallFunction|UpdateSeason))

(fn ComputeCurrentTime
  (bind _returnvalue (Utilities|Time|GetWorldDeltaSeconds))
  (bind _daylength (Variables|TimeSetup|GetDayLength))
  (bind _returnvalue_2 (* _daylength 6e+01))
  (bind _returnvalue_3 (/ _returnvalue_2 24.0))
  (bind _returnvalue_4 (Math|Float|SafeDivide _returnvalue _returnvalue_3))
  (LocalVariables|SetTempDayCycle (+ _returnvalue_4 (Variables|TimeSetup|GetDayCycleHour)))
  (LocalVariables|SetTempMoonCycle (+ _returnvalue_4 (Variables|TimeSetup|GetMoonCycleHour)))
  (Variables|TimeSetup|SetDayCycleHour (Math|Float|SelectFloat (LocalVariables|GetTempDayCycle) (Math|Float|Absolute(Float) (- 24.0 (LocalVariables|GetTempDayCycle))) (< (LocalVariables|GetTempDayCycle) 24.0)))
  (Variables|TimeSetup|SetMoonCycleHour (Math|Float|SelectFloat (LocalVariables|GetTempMoonCycle) (Math|Float|Absolute(Float) (- 25.0 (LocalVariables|GetTempMoonCycle))) (< (LocalVariables|GetTempMoonCycle) 25.0))))

(fn UpdateSunMoonPosition
  (params (SunHeight :type Float%20%28double-precision%29))
  (bind _returnvalue (Math|Float|MakeLiteralFloat 1.25))
  (bind _returnvalue_2 (Math|Float|MakeLiteralFloat 175.0))
  (bind _returnvalue_3 (Math|Float|MakeLiteralFloat 1.75))
  (bind _daycyclehour (Variables|TimeSetup|GetDayCycleHour))
  (bind _mooncyclehour (Variables|TimeSetup|GetMoonCycleHour))
  (Transformation|SetWorldRotation (Variables|Default|GetSun) (Math|Rotator|MakeRotator 0.0 (Math|Float|SelectFloat (Class|KismetMathLibrary|FInterpEaseinOut _returnvalue_2 SunHeight (Math|Float|SelectFloat (Math|Float|MapRangeClamped _daycyclehour (Variables|Season|GetSunriseTime) 12.0 0.0 1.0) (Math|Float|MapRangeClamped _daycyclehour 12.0 (Variables|Season|GetSunsetTime) 1.0 0.0) (< (Variables|TimeSetup|GetDayCycleHour) 12.0)) _returnvalue) (Class|KismetMathLibrary|FInterpEaseinOut _returnvalue_2 (- 3.6e+02 SunHeight) (Math|Float|SelectFloat (Math|Float|MapRangeClamped _daycyclehour (Variables|Season|GetSunsetTime) 24.0 0.0 1.0) (Math|Float|MapRangeClamped _daycyclehour 0.0 (Variables|Season|GetSunriseTime) 1.0 0.0) (> (Variables|TimeSetup|GetDayCycleHour) (Variables|Season|GetSunsetTime))) _returnvalue) (Math|Float|InRange(Float) (Variables|TimeSetup|GetDayCycleHour) (Variables|Season|GetSunriseTime) (Variables|Season|GetSunsetTime) false false)) (Class|KismetMathLibrary|FInterpEaseinOut 0.0 3.6e+02 (Math|Float|NormalizetoRange (Variables|TimeSetup|GetDayCycleHour) 0.0 24.0) _returnvalue_3)) false false)
  (Transformation|SetWorldRotation (Variables|Default|GetMoon) (Math|Rotator|MakeRotator 0.0 (Math|Float|SelectFloat (Class|KismetMathLibrary|FInterpEaseinOut _returnvalue_2 SunHeight (Math|Float|SelectFloat (Math|Float|MapRangeClamped _mooncyclehour 0.0 13.0 0.0 1.0) (Math|Float|MapRangeClamped _mooncyclehour 13.0 19.0 1.0 0.0) (< (Variables|TimeSetup|GetMoonCycleHour) 13.0)) _returnvalue) (Class|KismetMathLibrary|FInterpEaseinOut _returnvalue_2 (- 3.6e+02 SunHeight) (Math|Float|SelectFloat (Math|Float|MapRangeClamped _mooncyclehour 19.0 25.0 0.0 1.0) (Math|Float|MapRangeClamped _mooncyclehour 0.0 6.0 1.0 0.0) (> (Variables|TimeSetup|GetMoonCycleHour) 19.0)) _returnvalue) (Math|Float|InRange(Float) (Variables|TimeSetup|GetMoonCycleHour) 6.0 19.0 false false)) (Class|KismetMathLibrary|FInterpEaseinOut 0.0 3.6e+02 (Math|Float|NormalizetoRange (Variables|TimeSetup|GetMoonCycleHour) 0.0 25.0) _returnvalue_3)) false false))

(fn InitStardome
  (Niagara|SetNiagaraVariable(Float) (Variables|Default|GetStars) "DayLength" (Variables|TimeSetup|GetDayLength)))

(fn GetPartOfDay
  (if (Math|Float|InRange(Float) (Variables|TimeSetup|GetDayCycleHour) (Variables|Season|GetSunriseTime) 12.0 true false)
    (return "NewEnumerator0")
    (elif (Math|Float|InRange(Float) (Variables|TimeSetup|GetDayCycleHour) 12.0 (Variables|Season|GetSunsetTime) true false)
      (return "NewEnumerator1")
      (elif (Math|Float|InRange(Float) (Variables|TimeSetup|GetDayCycleHour) (Variables|Season|GetSunsetTime) 21.0 true false)
        (return "NewEnumerator2")
        (else
          (return "NewEnumerator3"))))))

(fn UpdateWeather
  (Variables|TimeSetup|SetDeltaTime (+ (/ (Variables|TimeSetup|GetUpdateFrequency) (/ (* (Variables|TimeSetup|GetDayLength) 6e+01) 24.0)) (Variables|TimeSetup|GetDayCycleHour)))
  (switch Utilities|FlowControl|Switch|SwitchonE_Seasons (Variables|Season|GetSeason)
    (:NewEnumerator0
      (Utilities|FlowControl|Sequence
        (:then_0
          (Variables|Season|SetSnowWeight 0)
          (CallFunction|ToggleSnow :!label _label))
        (:then_1
          (Variables|Season|SetRainWeight 2)
          (CallFunction|ToggleRain :!label _label_2))))
    (:NewEnumerator1
      (Utilities|FlowControl|Sequence
        (:then_0
          (Variables|Season|SetSnowWeight 0)
          (goto _label))
        (:then_1
          (Variables|Season|SetRainWeight 1)
          (goto _label_2))))
    (:NewEnumerator2
      (Utilities|FlowControl|Sequence
        (:then_0
          (Variables|Season|SetSnowWeight 1)
          (goto _label))
        (:then_1
          (Variables|Season|SetRainWeight 3)
          (goto _label_2))))
    (:NewEnumerator3
      (Utilities|FlowControl|Sequence
        (:then_0
          (Variables|Season|SetSnowWeight 4)
          (goto _label))
        (:then_1
          (Variables|Season|SetRainWeight 4)
          (goto _label_2))))))

(fn ToggleSnow
  (bind _snowschedule (Variables|Precipitation|GetSnowSchedule))
  (bind _returnvalue (Utilities|Array|LastIndex _snowschedule))
  (if (or (Variables|TimeSetup|GetbFirstLaunch) (>= (Variables|TimeSetup|GetDeltaTime) 24.0))
    (LocalVariables|SetSnowCount (Variables|Season|GetSnowWeight))
    (if (Variables|TimeSetup|GetbFirstLaunch)
      (Variables|TimeSetup|SetbFirstLaunch false))
    (if (!= (LocalVariables|GetSnowCount) 0)
      (LocalVariables|SetSnowPeriod (/ 24 (LocalVariables|GetSnowCount)))
      (Utilities|Array|Clear (Variables|Precipitation|GetSnowSchedule))
      (for _index (range 1 (LocalVariables|GetSnowCount))
        (LocalVariables|SetSnowPeriodMinBound (* (+ (- (LocalVariables|GetSnowCount) _index) 1) (LocalVariables|GetSnowPeriod)))
        (LocalVariables|SetSnowPeriodMaxBound (- (* (+ (- (LocalVariables|GetSnowCount) _index) 1) (LocalVariables|GetSnowPeriod)) (LocalVariables|GetSnowPeriod)))
        (LocalVariables|SetSnowEndHour (Math|Random|RandomIntegerinRange (/ (+ (LocalVariables|GetSnowPeriodMinBound) (LocalVariables|GetSnowPeriodMaxBound)) 2) (LocalVariables|GetSnowPeriodMinBound)))
        (LocalVariables|SetSnowStartHour (Math|Random|RandomIntegerinRange (LocalVariables|GetSnowPeriodMaxBound) (/ (+ (LocalVariables|GetSnowPeriodMinBound) (LocalVariables|GetSnowPeriodMaxBound)) 2)))
        (if (> (LocalVariables|GetSnowEndHour) (Math|Float|Truncate (Variables|TimeSetup|GetDayCycleHour)))
          (Utilities|Array|Add (Variables|Precipitation|GetSnowSchedule) (LocalVariables|GetSnowEndHour))
          (if (> (LocalVariables|GetSnowStartHour) (Math|Float|Truncate (Variables|TimeSetup|GetDayCycleHour)))
            (Utilities|Array|Add (Variables|Precipitation|GetSnowSchedule) (LocalVariables|GetSnowStartHour)))))
      (Variables|Precipitation|SetbSnow (> (Math|Integer|%(Integer) (Utilities|Array|Length (Variables|Precipitation|GetSnowSchedule)) 2) 0))
      (if true
        (Components|Activation|Activate (Variables|Default|GetSnowComponent) false)
        (Variables|Default|SetbIsSnowNow true)
        (Development|PrintString "Snow")
        (else
          (Components|Activation|Deactivate (Variables|Default|GetSnowComponent))
          (Variables|Default|SetbIsSnowNow false)
          (Development|PrintString "Dry")))
      (else
        (Components|Activation|Deactivate (Variables|Default|GetSnowComponent))
        (Variables|Default|SetbIsSnowNow false)
        (Development|PrintString "No Snow")))
    (elif (> (Utilities|Array|Length (Variables|Precipitation|GetSnowSchedule)) 0)
      (if (>= (Math|Float|Truncate (Variables|TimeSetup|GetDayCycleHour)) (Utilities|Array|Get(acopy) _snowschedule _returnvalue))
        (Utilities|FlowControl|Sequence
          (:then_0
            (Variables|Precipitation|SetbSnow (not (Variables|Precipitation|GetbSnow)))
            (if (Variables|Precipitation|GetbSnow)
              (Components|Activation|Activate (Variables|Default|GetSnowComponent) false)
              (Variables|Default|SetbIsSnowNow true)
              (Development|PrintString "Global Snow")
              (else
                (Components|Activation|Deactivate (Variables|Default|GetSnowComponent))
                (Variables|Default|SetbIsSnowNow false)
                (Development|PrintString "Global Dry"))))
          (:then_1
            (Utilities|Array|RemoveIndex (Variables|Precipitation|GetSnowSchedule) _returnvalue)))))))

(fn ToggleRain
  (bind _rainschedule (Variables|Precipitation|GetRainSchedule))
  (bind _returnvalue (Utilities|Array|LastIndex _rainschedule))
  (if (or (Variables|TimeSetup|GetbFirstLaunch) (>= (Variables|TimeSetup|GetDeltaTime) 24.0))
    (LocalVariables|SetRainCount (Variables|Season|GetRainWeight))
    (if (Variables|TimeSetup|GetbFirstLaunch)
      (Variables|TimeSetup|SetbFirstLaunch false))
    (if (!= (LocalVariables|GetRainCount) 0)
      (LocalVariables|SetRainPeriod (/ 24 (LocalVariables|GetRainCount)))
      (Utilities|Array|Clear (Variables|Precipitation|GetRainSchedule))
      (for _index (range 1 (LocalVariables|GetRainCount))
        (LocalVariables|SetRainPeriodMinBound (* (+ (- (LocalVariables|GetRainCount) _index) 1) (LocalVariables|GetRainPeriod)))
        (LocalVariables|SetRainPeriodMaxBound (- (* (+ (- (LocalVariables|GetRainCount) _index) 1) (LocalVariables|GetRainPeriod)) (LocalVariables|GetRainPeriod)))
        (LocalVariables|SetRainEndHour (Math|Random|RandomIntegerinRange (/ (+ (LocalVariables|GetRainPeriodMinBound) (LocalVariables|GetRainPeriodMaxBound)) 2) (LocalVariables|GetRainPeriodMinBound)))
        (LocalVariables|SetRainStartHour (Math|Random|RandomIntegerinRange (LocalVariables|GetRainPeriodMaxBound) (/ (+ (LocalVariables|GetRainPeriodMinBound) (LocalVariables|GetRainPeriodMaxBound)) 2)))
        (if (> (LocalVariables|GetRainEndHour) (Math|Float|Truncate (Variables|TimeSetup|GetDayCycleHour)))
          (Utilities|Array|Add (Variables|Precipitation|GetRainSchedule) (LocalVariables|GetRainEndHour))
          (if (> (LocalVariables|GetRainStartHour) (Math|Float|Truncate (Variables|TimeSetup|GetDayCycleHour)))
            (Utilities|Array|Add (Variables|Precipitation|GetRainSchedule) (LocalVariables|GetRainStartHour)))))
      (Variables|Precipitation|SetbRain (> (Math|Integer|%(Integer) (Utilities|Array|Length (Variables|Precipitation|GetRainSchedule)) 2) 0))
      (if true
        (Components|Activation|Activate (Variables|Default|GetRainComponent) false)
        (Variables|Default|SetbIsRainNow true)
        (Development|PrintString "Rain")
        (else
          (Components|Activation|Deactivate (Variables|Default|GetRainComponent))
          (Variables|Default|SetbIsRainNow false)
          (Development|PrintString "Dry")))
      (else
        (Components|Activation|Deactivate (Variables|Default|GetRainComponent))
        (Variables|Default|SetbIsRainNow false)
        (Development|PrintString "No Rain")))
    (elif (> (Utilities|Array|Length (Variables|Precipitation|GetRainSchedule)) 0)
      (if (>= (Math|Float|Truncate (Variables|TimeSetup|GetDayCycleHour)) (Utilities|Array|Get(acopy) _rainschedule _returnvalue))
        (Utilities|FlowControl|Sequence
          (:then_0
            (Variables|Precipitation|SetbRain (not (Variables|Precipitation|GetbRain)))
            (if (Variables|Precipitation|GetbRain)
              (Components|Activation|Activate (Variables|Default|GetRainComponent) false)
              (Variables|Default|SetbIsRainNow true)
              (Development|PrintString "Global Rain")
              (else
                (Components|Activation|Deactivate (Variables|Default|GetRainComponent))
                (Variables|Default|SetbIsRainNow false)
                (Development|PrintString "Global Dry"))))
          (:then_1
            (Utilities|Array|RemoveIndex (Variables|Precipitation|GetRainSchedule) _returnvalue)))))))

(fn UpdateDate
  (if (> (+ (Variables|TimeSetup|GetDay) 1) 30)
    (Variables|TimeSetup|SetDay 1)
    (if (> (+ (Variables|TimeSetup|GetMonth) 1) 12)
      (Variables|TimeSetup|SetMonth "NewEnumerator0")
      (else
        (Variables|TimeSetup|SetMonth (Utilities|Enum|ByteToEnumE_Month (+ (Variables|TimeSetup|GetMonth) 1)))))
    (CallFunction|UpdateSeason)
    (Variables|TimeSetup|SetYear (+ (Variables|TimeSetup|GetYear) 1))
    (else
      (Variables|TimeSetup|SetDay (+ (Variables|TimeSetup|GetDay) 1)))))

(fn UpdateSeason
  (switch Utilities|FlowControl|Switch|SwitchonE_Month (Variables|TimeSetup|GetMonth)
    (:NewEnumerator0
      (Variables|Season|SetSunriseTime 7.25)
      (Variables|Season|SetSunsetTime 17.0))
    (:NewEnumerator1
      (Variables|Season|SetSunriseTime 6.75)
      (Variables|Season|SetSunsetTime 17.5))
    (:NewEnumerator2
      (Variables|Season|SetSeason "NewEnumerator0")
      (Variables|Season|SetSunriseTime 6.0)
      (Variables|Season|SetSunsetTime 18.5))
    (:NewEnumerator3
      (Variables|Season|SetSunriseTime 5.75)
      (Variables|Season|SetSunsetTime 19.0))
    (:NewEnumerator4
      (Variables|Season|SetSunriseTime 5.5)
      (Variables|Season|SetSunsetTime 19.5))
    (:NewEnumerator11
      (Variables|Season|SetSeason "NewEnumerator1")
      (Variables|Season|SetSunriseTime 5.25)
      (Variables|Season|SetSunsetTime 2e+01))
    (:NewEnumerator5
      (Variables|Season|SetSunriseTime 5.5)
      (Variables|Season|SetSunsetTime 2e+01))
    (:NewEnumerator6
      (Variables|Season|SetSunriseTime 5.75)
      (Variables|Season|SetSunsetTime 19.5))
    (:NewEnumerator7
      (Variables|Season|SetSeason "NewEnumerator2")
      (Variables|Season|SetSunriseTime 6.0)
      (Variables|Season|SetSunsetTime 19.0))
    (:NewEnumerator8
      (Variables|Season|SetSunriseTime 6.25)
      (Variables|Season|SetSunsetTime 18.5))
    (:NewEnumerator9
      (Variables|Season|SetSunriseTime 6.5)
      (Variables|Season|SetSunsetTime 17.5))
    (:NewEnumerator10
      (Variables|Season|SetSeason "NewEnumerator3")
      (Variables|Season|SetSunriseTime 7.0)
      (Variables|Season|SetSunsetTime 16.5))))