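; BP_ToolBase is the base Blueprint for tool pickups that the player can add to an inventory.
; Its sphere overlap stores the overlapping actor and enables the tool's input for the player character, while end overlap calls DisableInput on the player controller.
; IA_Interact sends STools to the stored actor through AddToInventoryMessage and destroys the tool on success.
; LookAt returns a fixed name, and debug prints trace the overlaps.
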(event OnComponentBeginOverlap(Sphere)
  (params (OverlappedComponent :type Primitive%20Component%20Object%20Reference) (OtherActor :type Actor%20Object%20Reference) (OtherComp :type Primitive%20Component%20Object%20Reference) (OtherBodyIndex :type Integer) (bFromSweep :type Boolean) (SweepResult :type Hit%20Result%20Structure%20%28by%20ref%29))
  (Development|PrintString "SOMETHING IS OVERLAPPING")
  (Variables|Default|SetOther%20Actor OtherActor)
  (if (== OtherActor (Game|GetPlayerCharacter 0))
    (Development|PrintString "IS A PLAYER CHACRTYER")
    (Input|EnableInput (Game|GetPlayerController 0))
    (else
      (Development|PrintString "NOT A PLAYER CHARACTER"))))

(event OnComponentEndOverlap(Sphere)
  (params (OverlappedComponent :type Primitive%20Component%20Object%20Reference) (OtherActor :type Actor%20Object%20Reference) (OtherComp :type Primitive%20Component%20Object%20Reference) (OtherBodyIndex :type Integer))
  (if (== OtherActor (Game|GetPlayerCharacter 0))
    (Input|DisableInput (Game|GetPlayerController 0) 0)))

(event Input|EnhancedActionEvents|EnhancedInputActionIA_Interact
  (params (ActionValue :type Boolean) (ElapsedSeconds :type Float%20%28double-precision%29) (TriggeredSeconds :type Float%20%28double-precision%29) (InputAction :type Input%20Action%20Object%20Reference :default "/Game/VoxelGame/Input/Actions/IA_Interact.IA_Interact"))
  (:Started
    (bind _success (Class|BPIInventory|AddtoInventory(Message) (Variables|Default|GetOther%20Actor) (Variables|Default|GetS_Tools)))
    (if _success
      (Actor|DestroyActor))))

(event EventBeginPlay)

(event Collision|EventActorBeginOverlap
  (params (OtherActor :type Actor%20Object%20Reference)))

(event EventTick
  (params (DeltaSeconds :type Float%20%28single-precision%29)))

(fn ConstructionScript)

(fn Lookat
  (return "ToolBase"))