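; BP_VoxelGame_PlayerController is the voxel game's player controller, handling input mode and on-screen widgets.
; On BeginPlay it caches the third-person character, sets game-only input with a hidden cursor, and creates the HUD for the local player.
; Separate events create a time widget fed by a weather system and remove it.
; The DestroyTimeWidget function is an empty stub, while removal runs in the DestroyTimeWidget_1_1 event.
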(event Custom|DestroyTimeWidget_1_1
  (params (WeatherSystem :type BP%20Sky%20Manager%20Object%20Reference))
  (Utilities|IsValid (Variables|Default|GetGUI_Time)
    (:Is%20Valid
      (Widget|RemovefromParent (Variables|Default|GetGUI_Time))
      (Variables|Default|SetGUI_Time 0))))

(event EventBeginPlay
  (bind _self self)
  (bind _asbp_third_person_character (Utilities|Casting|CastToBP_ThirdPersonCharacter (Game|GetPlayerCharacter 0)))
  (Variables|Default|SetThirdPersonCharacterReference _asbp_third_person_character)
  (Input|SetInputModeGameOnly _self false)
  (Variables|Default|SetbShowMouseCursor _self false)
  (if (Pawn|IsLocalPlayerController)
    ;[1 1 1] Create HUD
    (bind _returnvalue (UserInterface|CreateWidget "/Game/VoxelGame/Blueprints/UI/WBP_HUD.WBP_HUD_C"))
    (bind _output_get (Variables|Default|SetHudReference _returnvalue))
    (UserInterface|Viewport|AddtoViewport _output_get 0)))

(event EventCreateTimeWidget
  (params (WeatherSystem :type BP%20Sky%20Manager%20Object%20Reference))
  (bind _returnvalue (UserInterface|CreateWidget "/Game/VoxelGame/Blueprints/UI/WBP_HUD-Time.WBP_HUD-Time_C" 0 WeatherSystem))
  (bind _output_get (Variables|Default|SetGUI_Time _returnvalue))
  (UserInterface|Viewport|AddtoViewport _output_get 0))

(fn ConstructionScript)

(fn DestroyTimeWidget
  (params (WeatherSystem :type BP%20Sky%20Manager%20Object%20Reference))
  (return "Null"))