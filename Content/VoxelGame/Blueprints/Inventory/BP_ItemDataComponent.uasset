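; BP_ItemDataComponent turns its owning actor into an item that a player can pick up, holding an item row reference and quantity.
; On BeginPlay it sets the owner to replicate.
; Interactwith passes the item's row name and quantity to the player's InventorySystem and destroys the owner only if the add succeeds.
; LookAt currently returns an empty string.
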(event EventBeginPlay
  (Networking|SetReplicates (Components|GetOwner) true))

(event EventInteractwith
  (params (PlayerCharacter :type BP%20Third%20Person%20Character%20Object%20Reference))
  (bind _inventorysystem (Variables|/Game/VoxelGame/Blueprints/Core/BP_ThirdPersonCharacter.BP_ThirdPersonCharacter_C|GetInventorySystem PlayerCharacter))
  (Utilities|IsValid _inventorysystem
    (:Is%20Valid
      (bind _success (Default|AddtoInventory _inventorysystem (.rowname (Variables|Default|GetItemID)) (Variables|Default|GetQuantity)))
      (if _success
        (Actor|DestroyActor (Components|GetOwner))))))

(fn Lookat
  (return ""))