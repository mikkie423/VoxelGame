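; Dropped item actor for a terrain block in the voxel game, showing that block type's texture on a cube.
; On BeginPlay, SetItemData maps BlockType to a DT_ItemData row handle on ItemDataComponent, with Air and Null falling back to apple.
; The row's MaterialIndex then drives TextureIndex on a dynamic texture-array material instance.
; LookAt returns the item's name from the same table.
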(event EventBeginPlay
  (CallFunction|SetItemData (Variables|Default|GetBlockType))
  (bind _returnvalue (Utilities|GetDataTableRow "/Game/VoxelGame/Blueprints/Inventory/DT_ItemData.DT_ItemData" (.rowname (Variables|/Game/VoxelGame/Blueprints/Inventory/BP_ItemDataComponent.BP_ItemDataComponent_C|GetItemID (Variables|Default|GetItemDataComponent))))
    (:then
      (Development|PrintString (Utilities|String|Append "Dropping " (Utilities|String|ToString(Text) (.name _returnvalue)) " MaterialIndex: " (Utilities|String|ToString(Integer) (.materialindex _returnvalue))))
      (Variables|Default|SetBlockType (.blocktype _returnvalue))
      (CallFunction|SetMaterial (.materialindex _returnvalue)))
    (:RowNotFound
      (Development|PrintString "ROW NOT FOUND" true true "(R=1.000000,G=0.000000,B=0.102836,A=1.000000)"))))

(event EventTick
  (params (DeltaSeconds :type Float%20%28single-precision%29)))

(event EventSetMaterial
  (params (MaterialIndex :type Integer))
  (bind _cube (Variables|Default|GetCube))
  (bind _returnvalue (Rendering|Material|CreateDynamicMaterialInstance _cube 0 "/Game/VoxelGame/Blueprints/Terrain/M_TerrainItemTextureArray.M_TerrainItemTextureArray" "None" :!class /Script/Engine.PrimitiveComponent))
  (Rendering|Material|SetScalarParameterValue _returnvalue "TextureIndex" (Math|Conversions|ToFloat(Integer) MaterialIndex) :!class /Script/Engine.MaterialInstanceDynamic)
  (Rendering|Material|SetMaterial _cube MaterialIndex _returnvalue))

(fn ConstructionScript)

(fn SetItemData
  (params (BlockType :type EBlock%20Enum :default "Grass"))
  (switch Utilities|FlowControl|Switch|SwitchonEBlock BlockType
    (:Grass
      (bind _output_get (Variables|/Game/VoxelGame/Blueprints/Inventory/BP_ItemDataComponent.BP_ItemDataComponent_C|SetItemID (Variables|Default|GetItemDataComponent) (Utilities|Struct|MakeDataTableRowHandle "/Game/VoxelGame/Blueprints/Inventory/DT_ItemData.DT_ItemData" "grass")))
      (Utilities|Struct|SetmembersinDataTableRowHandle _output_get))
    (:Dirt
      (bind _output_get_2 (Variables|/Game/VoxelGame/Blueprints/Inventory/BP_ItemDataComponent.BP_ItemDataComponent_C|SetItemID (Variables|Default|GetItemDataComponent) (Utilities|Struct|MakeDataTableRowHandle "/Game/VoxelGame/Blueprints/Inventory/DT_ItemData.DT_ItemData" "dirt")))
      (Utilities|Struct|SetmembersinDataTableRowHandle _output_get_2))
    (:Stone
      (bind _output_get_3 (Variables|/Game/VoxelGame/Blueprints/Inventory/BP_ItemDataComponent.BP_ItemDataComponent_C|SetItemID (Variables|Default|GetItemDataComponent) (Utilities|Struct|MakeDataTableRowHandle "/Game/VoxelGame/Blueprints/Inventory/DT_ItemData.DT_ItemData" "stone")))
      (Utilities|Struct|SetmembersinDataTableRowHandle _output_get_3))
    (:Bedrock
      (bind _output_get_4 (Variables|/Game/VoxelGame/Blueprints/Inventory/BP_ItemDataComponent.BP_ItemDataComponent_C|SetItemID (Variables|Default|GetItemDataComponent) (Utilities|Struct|MakeDataTableRowHandle "/Game/VoxelGame/Blueprints/Inventory/DT_ItemData.DT_ItemData" "bedrock")))
      (Utilities|Struct|SetmembersinDataTableRowHandle _output_get_4))
    (:Log
      (bind _output_get_5 (Variables|/Game/VoxelGame/Blueprints/Inventory/BP_ItemDataComponent.BP_ItemDataComponent_C|SetItemID (Variables|Default|GetItemDataComponent) (Utilities|Struct|MakeDataTableRowHandle "/Game/VoxelGame/Blueprints/Inventory/DT_ItemData.DT_ItemData" "log")))
      (Utilities|Struct|SetmembersinDataTableRowHandle _output_get_5))
    (:Leaves
      (bind _output_get_6 (Variables|/Game/VoxelGame/Blueprints/Inventory/BP_ItemDataComponent.BP_ItemDataComponent_C|SetItemID (Variables|Default|GetItemDataComponent) (Utilities|Struct|MakeDataTableRowHandle "/Game/VoxelGame/Blueprints/Inventory/DT_ItemData.DT_ItemData" "leaves")))
      (Utilities|Struct|SetmembersinDataTableRowHandle _output_get_6))
    (:Sand
      (bind _output_get_7 (Variables|/Game/VoxelGame/Blueprints/Inventory/BP_ItemDataComponent.BP_ItemDataComponent_C|SetItemID (Variables|Default|GetItemDataComponent) (Utilities|Struct|MakeDataTableRowHandle "/Game/VoxelGame/Blueprints/Inventory/DT_ItemData.DT_ItemData" "sand")))
      (Utilities|Struct|SetmembersinDataTableRowHandle _output_get_7))
    (:Gravel
      (bind _output_get_8 (Variables|/Game/VoxelGame/Blueprints/Inventory/BP_ItemDataComponent.BP_ItemDataComponent_C|SetItemID (Variables|Default|GetItemDataComponent) (Utilities|Struct|MakeDataTableRowHandle "/Game/VoxelGame/Blueprints/Inventory/DT_ItemData.DT_ItemData" "gravel")))
      (Utilities|Struct|SetmembersinDataTableRowHandle _output_get_8))
    (:ShallowWater
      (bind _output_get_9 (Variables|/Game/VoxelGame/Blueprints/Inventory/BP_ItemDataComponent.BP_ItemDataComponent_C|SetItemID (Variables|Default|GetItemDataComponent) (Utilities|Struct|MakeDataTableRowHandle "/Game/VoxelGame/Blueprints/Inventory/DT_ItemData.DT_ItemData" "shallowWater")))
      (Utilities|Struct|SetmembersinDataTableRowHandle _output_get_9))
    (:DeepWater
      (bind _output_get_10 (Variables|/Game/VoxelGame/Blueprints/Inventory/BP_ItemDataComponent.BP_ItemDataComponent_C|SetItemID (Variables|Default|GetItemDataComponent) (Utilities|Struct|MakeDataTableRowHandle "/Game/VoxelGame/Blueprints/Inventory/DT_ItemData.DT_ItemData" "deepWater")))
      (Utilities|Struct|SetmembersinDataTableRowHandle _output_get_10))
    (:Swamp
      (bind _output_get_11 (Variables|/Game/VoxelGame/Blueprints/Inventory/BP_ItemDataComponent.BP_ItemDataComponent_C|SetItemID (Variables|Default|GetItemDataComponent) (Utilities|Struct|MakeDataTableRowHandle "/Game/VoxelGame/Blueprints/Inventory/DT_ItemData.DT_ItemData" "swamp")))
      (Utilities|Struct|SetmembersinDataTableRowHandle _output_get_11))
    (:Taiga
      (bind _output_get_12 (Variables|/Game/VoxelGame/Blueprints/Inventory/BP_ItemDataComponent.BP_ItemDataComponent_C|SetItemID (Variables|Default|GetItemDataComponent) (Utilities|Struct|MakeDataTableRowHandle "/Game/VoxelGame/Blueprints/Inventory/DT_ItemData.DT_ItemData" "taiga")))
      (Utilities|Struct|SetmembersinDataTableRowHandle _output_get_12))
    (:Tundra
      (bind _output_get_13 (Variables|/Game/VoxelGame/Blueprints/Inventory/BP_ItemDataComponent.BP_ItemDataComponent_C|SetItemID (Variables|Default|GetItemDataComponent) (Utilities|Struct|MakeDataTableRowHandle "/Game/VoxelGame/Blueprints/Inventory/DT_ItemData.DT_ItemData" "tundra")))
      (Utilities|Struct|SetmembersinDataTableRowHandle _output_get_13))
    (:Ice
      (bind _output_get_14 (Variables|/Game/VoxelGame/Blueprints/Inventory/BP_ItemDataComponent.BP_ItemDataComponent_C|SetItemID (Variables|Default|GetItemDataComponent) (Utilities|Struct|MakeDataTableRowHandle "/Game/VoxelGame/Blueprints/Inventory/DT_ItemData.DT_ItemData" "ice")))
      (Utilities|Struct|SetmembersinDataTableRowHandle _output_get_14))
    (:Air
      (bind _output_get_15 (Variables|/Game/VoxelGame/Blueprints/Inventory/BP_ItemDataComponent.BP_ItemDataComponent_C|SetItemID (Variables|Default|GetItemDataComponent) (Utilities|Struct|MakeDataTableRowHandle "/Game/VoxelGame/Blueprints/Inventory/DT_ItemData.DT_ItemData" "apple") :!label _label))
      (Utilities|Struct|SetmembersinDataTableRowHandle _output_get_15))
    (:Null
      (goto _label))))

(fn Lookat
  (bind _itemdatacomponent (Variables|Default|GetItemDataComponent))
  (bind _itemid (Variables|/Game/VoxelGame/Blueprints/Inventory/BP_ItemDataComponent.BP_ItemDataComponent_C|GetItemID _itemdatacomponent))
  (bind _returnvalue (Utilities|GetDataTableRow (.datatable _itemid) (.rowname _itemid))
    (:then
      (return (Utilities|Text|FormatText "{item}" (.Name (Utilities|Struct|BreakF_ItemStruct _returnvalue)))))))