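; Game instance for the voxel game that manages the save slot and holds the current world's seed and name.
; Init and SaveGame share one path that loads or creates a BP_SaveGame, then writes it straight back without copying world values into it.
; LoadGame reads an existing slot and copies WorldSeed and WorldName from the save object into the instance.
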(event Custom|LoadGame
  (params (SaveGameName :type String))
  (bind _returnvalue (SaveGame|DoesSaveGameExist SaveGameName))
  (if _returnvalue
    (bind _returnvalue_2 (SaveGame|LoadGamefromSlot SaveGameName))
    (bind _asbp_save_game (Utilities|Casting|CastToBP_SaveGame _returnvalue_2))
    (bind _output_get (Variables|Default|SetSaveVar _asbp_save_game))
    (Variables|Default|SetWorld%20Seed (Variables|/Game/VoxelGame/Core/BP_SaveGame.BP_SaveGame_C|GetWorldSeed _output_get))
    (Variables|Default|SetWorld%20Name (Variables|/Game/VoxelGame/Core/BP_SaveGame.BP_SaveGame_C|GetWorldName _output_get))))

(event Custom|SaveGame
  (params (SaveGameName :type String))
  (bind _returnvalue (SaveGame|DoesSaveGameExist SaveGameName))
  (if _returnvalue
    (bind _returnvalue_2 (SaveGame|LoadGamefromSlot SaveGameName))
    (bind _asbp_save_game (Utilities|Casting|CastToBP_SaveGame _returnvalue_2))
    (Variables|Default|SetSaveVar _asbp_save_game)
    (else
      (bind _returnvalue_3 (SaveGame|CreateSaveGameObject "/Game/VoxelGame/Core/BP_SaveGame.BP_SaveGame_C"))
      (Variables|Default|SetSaveVar _returnvalue_3)))
  (SaveGame|SaveGametoSlot (Variables|Default|GetSaveVar) SaveGameName))

(event EventInit
  (bind _returnvalue (SaveGame|DoesSaveGameExist (stale Custom|SaveGame SaveGameName)))
  (if _returnvalue
    (bind _returnvalue_2 (SaveGame|LoadGamefromSlot (stale Custom|SaveGame SaveGameName)))
    (bind _asbp_save_game (Utilities|Casting|CastToBP_SaveGame _returnvalue_2))
    (Variables|Default|SetSaveVar _asbp_save_game)
    (else
      (bind _returnvalue_3 (SaveGame|CreateSaveGameObject "/Game/VoxelGame/Core/BP_SaveGame.BP_SaveGame_C"))
      (Variables|Default|SetSaveVar _returnvalue_3)))
  (SaveGame|SaveGametoSlot (Variables|Default|GetSaveVar) (stale Custom|SaveGame SaveGameName)))