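; Player controller for the voxel game that sets up local player input and the HUD when play begins.
; On BeginPlay it caches player 0's third-person character, stopping if the cast fails, then switches to game-only input with a hidden cursor.
; For local controllers it creates the HUD widget, stores a reference and adds it to the viewport.
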(event EventBeginPlay
  (bind _self self)
  (bind _asbp_third_person_character (Utilities|Casting|CastToBP_ThirdPersonCharacter (Game|GetPlayerCharacter 0)))
  (Variables|Default|SetThirdPersonCharacterReference _asbp_third_person_character)
  (Input|SetInputModeGameOnly _self false)
  (Variables|Default|SetbShowMouseCursor _self false)
  (if (Pawn|IsLocalPlayerController)
    ;[1 1 1] Create HUD
    (bind _returnvalue (UserInterface|CreateWidget "/Game/VoxelGame/Blueprints/Inventory/UI/WBP_HUD.WBP_HUD_C"))
    (bind _output_get (Variables|Default|SetHudReference _returnvalue))
    (UserInterface|Viewport|AddtoViewport _output_get 0)))

(fn ConstructionScript)